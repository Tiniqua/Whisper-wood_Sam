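; AI controller for a Wisp character that has home and work buildings.
; On BeginPlay it runs the Dev_Behaviour behavior tree, and its setters write the home building, home spawn point and work building to the Blackboard.
; SetWorkLocation also caches the work building, while the UpdateWorkBuilding event writes only the Blackboard key.
; SetIsWorking stores a controller flag without writing it to the Blackboard.
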(event `self.ReceiveBeginPlay`
  (`self.RunBehaviorTree` "/Game/AI/Dev_Behaviour.Dev_Behaviour"))

(event `self.UpdateWorkBuilding`
  (params (WorkBuilding :type "Actor Object Reference"))
  (`BlackboardComponent.SetValueAsObject` (`AIBlueprintHelperLibrary.GetBlackboard` null) "WorkBuilding" WorkBuilding))

(fn `SetHomeLocation`
  (params (HomeReference :type "BaseBuilding Object Reference") (HomeSpawnLocation :type "Vector Structure"))
  (`BlackboardComponent.SetValueAsObject` (`AIBlueprintHelperLibrary.GetBlackboard` null) "HomeBuilding" HomeReference)
  (`BlackboardComponent.SetValueAsVector` (`AIBlueprintHelperLibrary.GetBlackboard` null) "HomeSpawnPoint" HomeSpawnLocation))

(fn `SetIsWorking`
  (params (IsWorking :type Boolean))
  (set `self.IsWorking` IsWorking))

(fn `SetWorkLocation`
  (params (WorkLocation :type "BaseBuilding Object Reference"))
  (bind _output_get (set `self.WorkBuilding` WorkLocation))
  (`BlackboardComponent.SetValueAsObject` (`AIBlueprintHelperLibrary.GetBlackboard` null) "WorkBuilding" _output_get))

(fn `UserConstructionScript`)