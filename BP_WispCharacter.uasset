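; BP_WispCharacter is the character Blueprint for a Wisp, an AI-controlled unit with happiness data and a job building.
; On BeginPlay it caches its BP_WispAIController, which supplies the current work building and workstation data.
; When ShouldDrawDebug is set, Tick calls DrawDebug to stack floating text above it showing happiness, job building and workstation key, using DeltaSeconds as duration so the text refreshes each frame.
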(event `self.ReceiveBeginPlay`
  (bind _asbp_wisp_aicontroller (cast `/Game/AI/Blueprints/BP_WispAIController` (`AIBlueprintHelperLibrary.GetAIController` self)))
  (set `self.Wisp AIController` _asbp_wisp_aicontroller))

(event `self.ReceiveTick`
  (params (DeltaSeconds :type "Float (single-precision)"))
  (if (`self.ShouldDrawDebug`)
    (`self.DrawDebug` DeltaSeconds)))

(fn `DrawDebug`
  (params (InputPin :type "Float (single-precision)"))
  (bind (_returnvalue_x _returnvalue_y _returnvalue_z) (`KismetMathLibrary.BreakVector` (`self.K2_GetActorLocation`)))
  (bind _wisp_aicontroller (`self.Wisp AIController`))
  (bind _wispdata_happiness (break `WispData` (`self.WispData`)))
  (bind (_workstationdata_bisoccupied _workstationdata_location _workstationdata_workstationkey) (break `Workstation` (`WispAIController.WorkstationData` _wisp_aicontroller)))
  (bind _returnvalue (`KismetMathLibrary.MakeVector` _returnvalue_x _returnvalue_y (+ _returnvalue_z 80.0)))
  (bind _returnvalue_2 (+ _returnvalue (0.0 0.0 20.0)))
  (`KismetSystemLibrary.DrawDebugString` _returnvalue (`KismetStringLibrary.Concat_StrStr` "Happiness:" (`KismetStringLibrary.Conv_DoubleToString` _wispdata_happiness)) null (struct :`A` 1.0) InputPin)
  (`KismetSystemLibrary.DrawDebugString` _returnvalue_2 (`KismetStringLibrary.Concat_StrStr` "Job Building:" (`KismetSystemLibrary.GetDisplayName` (`WispAIController.CurrentWorkBuilding` _wisp_aicontroller))) null (struct :`A` 1.0) InputPin)
  (`KismetSystemLibrary.DrawDebugString` (+ _returnvalue_2 (0.0 0.0 20.0)) (`KismetStringLibrary.Concat_StrStr` "Workstation Key:" (`KismetStringLibrary.Conv_IntToString` _workstationdata_workstationkey)) null (struct :`A` 1.0) InputPin))

(fn `UserConstructionScript`)